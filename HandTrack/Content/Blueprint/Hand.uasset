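; Hand Blueprint that physically simulates a skeletal mesh and grips its bones with physics handles, driven by a landmark-to-coordinate bone mapping.
; Every Tick enables physics on all bodies, then creates a new physics handle for each mapping entry and grabs that landmark's bone.
; Each handle targets the bone's current socket location, and mapped coordinates go into Grab rather than the target.
; A SocketIO client reference is left unused.
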(event `self.ReceiveTick`
  (params (DeltaSeconds :type "Float (single-precision)"))
  (`SkeletalMeshComponent.SetAllBodiesSimulatePhysics` (`self.SkeletalMesh`) true)
  (for _array_element (`self.BoneMapping`)
    (bind _returnvalue (`AddComponent|NODE_AddPhysicsHandleComponent-0`))
    (bind (_landmark _coordinates) (break `/Game/Blueprint/BoneMap` _array_element))
    (`BlueprintMapLibrary.Map_Add` (`self.grab`) _coordinates)
    (bind _returnvalue_2 (`SceneComponent.GetSocketLocation` (`self.SkeletalMesh`) _landmark))
    (`PhysicsHandleComponent.GrabComponentAtLocation` _returnvalue (`self.SkeletalMesh`) _landmark _returnvalue_2)
    (`PhysicsHandleComponent.SetTargetLocation` _returnvalue _returnvalue_2)))

(fn `UserConstructionScript`)