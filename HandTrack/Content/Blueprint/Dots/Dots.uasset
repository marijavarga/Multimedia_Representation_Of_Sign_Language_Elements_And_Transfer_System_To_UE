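; Dots is a Blueprint with a SocketIO client that receives hand-landmark data as JSON and prints it for debugging.
; On a "new wind" event it parses the message and prints selected thumb and wrist coordinates, along with a test string.
; Connection and disconnection are also printed.
; Logic to rotate the Wrist component from the received data is present but disconnected, so nothing moves.
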(event `self.SocketIOClient.OnGenericEvent`
  (params (EventName :type String) (MessageJson :type "SIOJsonValue Object Reference"))
  (if (`KismetStringLibrary.EqualEqual_StrStr` EventName "new wind")
    (bind _returnvalue (`EasyJsonParseManager.LoadFromString` (`SIOJsonValue.AsString` MessageJson))
      (:`Successed`
        (`KismetSystemLibrary.PrintString` (`EasyJsonObject.ReadString` _returnvalue "thumb_cmc.x" ""))
        (`KismetSystemLibrary.PrintString` "Hello")
        (`KismetSystemLibrary.PrintString` (`EasyJsonObject.ReadString` _returnvalue "wrist.y" ""))
        (`KismetSystemLibrary.PrintString` (`EasyJsonObject.ReadString` _returnvalue "wrist.z" ""))))))

(event `self.SocketIOClient.OnConnected`
  (params (SessionId :type String) (bIsReconnection :type Boolean))
  (`KismetSystemLibrary.PrintString` "Connected"))

(event `self.SocketIOClient.OnDisconnected`
  (params (Reason :type "ESIOConnectionCloseReason Enum" :default "CLOSE_REASON_NORMAL"))
  (`KismetSystemLibrary.PrintString` (`KismetStringLibrary.Concat_StrStr` "Disconnected" (`|GetEnumeratorNameAsString` Reason))))

(fn `UserConstructionScript`)