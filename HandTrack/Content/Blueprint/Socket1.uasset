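; Socket1 actor mirrors hand-landmark positions streamed over SocketIO onto per-joint components.
; BeginPlay binds the "new wind" event, whose JSON is parsed with EasyJsonParser.
; Each landmark's x/y/z is scaled, by 10 or by 2 for the wrist and some thumb joints, then applied instantly via MoveComponentTo.
; An Init routine pinning skeletal-mesh bones to target positions with physics handles exists but is never reached.
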(event `self.ReceiveBeginPlay`
  (`SocketIOClientComponent.BindEventToGenericEvent` (`self.SocketIOClient`) "new wind" "/"))

(event `self.ReceiveTick`
  (params (DeltaSeconds :type "Float (single-precision)")))

(event `self.SocketIOClient.OnConnected`
  (params (SessionId :type String) (bIsReconnection :type Boolean))
  (`KismetSystemLibrary.PrintString` "Connected"))

(event `self.SocketIOClient.OnDisconnected`
  (params (Reason :type "ESIOConnectionCloseReason Enum" :default "CLOSE_REASON_NORMAL"))
  (`KismetSystemLibrary.PrintString` (`KismetStringLibrary.Concat_StrStr` "Disconnected" (`|GetEnumeratorNameAsString` Reason))))

(event `self.SocketIOClient.OnGenericEvent`
  (params (EventName :type String) (MessageJson :type "SIOJsonValue Object Reference"))
  ;[1 1 1] SocketIO i EasyJsonParser plaginovi
  (if (`KismetStringLibrary.EqualEqual_StrStr` EventName "new wind")
    (bind _returnvalue (`EasyJsonParseManager.LoadFromString` (`SIOJsonValue.AsString` MessageJson))
      (:`Successed`
        (`KismetSystemLibrary.PrintString` "Hello")
        (`KismetSystemLibrary.MoveComponentTo` (`self.wrist`) (`KismetMathLibrary.MakeVector` (* (`KismetStringLibrary.Conv_StringToDouble` (`EasyJsonObject.ReadString` _returnvalue "wrist.x" "")) 2.0) (* (`KismetStringLibrary.Conv_StringToDouble` (`EasyJsonObject.ReadString` _returnvalue "wrist.y" "")) 2.0) (* (`KismetStringLibrary.Conv_StringToDouble` (`EasyJsonObject.ReadString` _returnvalue "wrist.z" "")) 2.0)) (struct) false false 0.0)
        (`KismetSystemLibrary.MoveComponentTo` (`self.thumb_cmc`) (`KismetMathLibrary.MakeVector` (* (`KismetStringLibrary.Conv_StringToDouble` (`EasyJsonObject.ReadString` _returnvalue "thumb_cmc.x" "")) 2.0) (* (`KismetStringLibrary.Conv_StringToDouble` (`EasyJsonObject.ReadString` _returnvalue "thumb_cmc.y" "")) 2.0) (* (`KismetStringLibrary.Conv_StringToDouble` (`EasyJsonObject.ReadString` _returnvalue "thumb_cmc.z" "")) 2.0)) (struct) false false 0.0)
        (`KismetSystemLibrary.MoveComponentTo` (`self.thumb_mcp`) (`KismetMathLibrary.MakeVector` (* (`KismetStringLibrary.Conv_StringToDouble` (`EasyJsonObject.ReadString` _returnvalue "thumb_mcp.x" "")) 2.0) (* (`KismetStringLibrary.Conv_StringToDouble` (`EasyJsonObject.ReadString` _returnvalue "thumb_mcp.y" "")) 2.0) (* (`KismetStringLibrary.Conv_StringToDouble` (`EasyJsonObject.ReadString` _returnvalue "thumb_mcp.z" "")) 2.0)) (struct) false false 0.0)
        (`KismetSystemLibrary.MoveComponentTo` (`self.thumb_ip`) (`KismetMathLibrary.MakeVector` (* (`KismetStringLibrary.Conv_StringToDouble` (`EasyJsonObject.ReadString` _returnvalue "thumb_ip.x" "")) 10.0) (* (`KismetStringLibrary.Conv_StringToDouble` (`EasyJsonObject.ReadString` _returnvalue "thumb_ip.y" "")) 10.0) (* (`KismetStringLibrary.Conv_StringToDouble` (`EasyJsonObject.ReadString` _returnvalue "thumb_ip.z" "")) 10.0)) (struct) false false 0.0)
        (`KismetSystemLibrary.MoveComponentTo` (`self.thumb_tip`) (`KismetMathLibrary.MakeVector` (* (`KismetStringLibrary.Conv_StringToDouble` (`EasyJsonObject.ReadString` _returnvalue "thumb_tip.x" "")) 2.0) (* (`KismetStringLibrary.Conv_StringToDouble` (`EasyJsonObject.ReadString` _returnvalue "thumb_tip.y" "")) 2.0) (* (`KismetStringLibrary.Conv_StringToDouble` (`EasyJsonObject.ReadString` _returnvalue "thumb_tip.z" "")) 2.0)) (struct) false false 0.0)
        (`KismetSystemLibrary.MoveComponentTo` (`self.index_finger_mcp`) (`KismetMathLibrary.MakeVector` (* (`KismetStringLibrary.Conv_StringToDouble` (`EasyJsonObject.ReadString` _returnvalue "index_finger_mcp.x" "")) 10.0) (* (`KismetStringLibrary.Conv_StringToDouble` (`EasyJsonObject.ReadString` _returnvalue "index_finger_mcp.y" "")) 10.0) (* (`KismetStringLibrary.Conv_StringToDouble` (`EasyJsonObject.ReadString` _returnvalue "index_finger_mcp.z" "")) 10.0)) (struct) false false 0.0)
        (`KismetSystemLibrary.MoveComponentTo` (`self.index_finger_pip`) (`KismetMathLibrary.MakeVector` (* (`KismetStringLibrary.Conv_StringToDouble` (`EasyJsonObject.ReadString` _returnvalue "index_finger_pip.x" "")) 10.0) (* (`KismetStringLibrary.Conv_StringToDouble` (`EasyJsonObject.ReadString` _returnvalue "index_finger_pip.y" "")) 10.0) (* (`KismetStringLibrary.Conv_StringToDouble` (`EasyJsonObject.ReadString` _returnvalue "index_finger_pip.z" "")) 10.0)) (struct) false false 0.0)
        (`KismetSystemLibrary.MoveComponentTo` (`self.index_finger_dip`) (`KismetMathLibrary.MakeVector` (* (`KismetStringLibrary.Conv_StringToDouble` (`EasyJsonObject.ReadString` _returnvalue "index_finger_dip.x" "")) 10.0) (* (`KismetStringLibrary.Conv_StringToDouble` (`EasyJsonObject.ReadString` _returnvalue "index_finger_dip.y" "")) 10.0) (* (`KismetStringLibrary.Conv_StringToDouble` (`EasyJsonObject.ReadString` _returnvalue "index_finger_dip.z" "")) 10.0)) (struct) false false 0.0)
        (`KismetSystemLibrary.MoveComponentTo` (`self.index_finger_tip`) (`KismetMathLibrary.MakeVector` (* (`KismetStringLibrary.Conv_StringToDouble` (`EasyJsonObject.ReadString` _returnvalue "index_finger_tip.x" "")) 10.0) (* (`KismetStringLibrary.Conv_StringToDouble` (`EasyJsonObject.ReadString` _returnvalue "index_finger_tip.y" "")) 10.0) (* (`KismetStringLibrary.Conv_StringToDouble` (`EasyJsonObject.ReadString` _returnvalue "index_finger_tip.z" "")) 10.0)) (struct) false false 0.0)
        (`KismetSystemLibrary.MoveComponentTo` (`self.middle_finger_mcp`) (`KismetMathLibrary.MakeVector` (* (`KismetStringLibrary.Conv_StringToDouble` (`EasyJsonObject.ReadString` _returnvalue "middle_finger_mcp.x" "")) 10.0) (* (`KismetStringLibrary.Conv_StringToDouble` (`EasyJsonObject.ReadString` _returnvalue "middle_finger_mcp.y" "")) 10.0) (* (`KismetStringLibrary.Conv_StringToDouble` (`EasyJsonObject.ReadString` _returnvalue "middle_finger_mcp.z" "")) 10.0)) (struct) false false 0.0)
        (`KismetSystemLibrary.MoveComponentTo` (`self.middle_finger_pip`) (`KismetMathLibrary.MakeVector` (* (`KismetStringLibrary.Conv_StringToDouble` (`EasyJsonObject.ReadString` _returnvalue "middle_finger_pip.x" "")) 10.0) (* (`KismetStringLibrary.Conv_StringToDouble` (`EasyJsonObject.ReadString` _returnvalue "middle_finger_pip.y" "")) 10.0) (* (`KismetStringLibrary.Conv_StringToDouble` (`EasyJsonObject.ReadString` _returnvalue "middle_finger_pip.z" "")) 10.0)) (struct) false false 0.0)
        (`KismetSystemLibrary.MoveComponentTo` (`self.middle_finger_dip`) (`KismetMathLibrary.MakeVector` (* (`KismetStringLibrary.Conv_StringToDouble` (`EasyJsonObject.ReadString` _returnvalue "middle_finger_dip.x" "")) 10.0) (* (`KismetStringLibrary.Conv_StringToDouble` (`EasyJsonObject.ReadString` _returnvalue "middle_finger_dip.y" "")) 10.0) (* (`KismetStringLibrary.Conv_StringToDouble` (`EasyJsonObject.ReadString` _returnvalue "middle_finger_dip.z" "")) 10.0)) (struct) false false 0.0)
        (`KismetSystemLibrary.MoveComponentTo` (`self.middle_finger_tip`) (`KismetMathLibrary.MakeVector` (* (`KismetStringLibrary.Conv_StringToDouble` (`EasyJsonObject.ReadString` _returnvalue "middle_finger_tip.x" "")) 10.0) (* (`KismetStringLibrary.Conv_StringToDouble` (`EasyJsonObject.ReadString` _returnvalue "middle_finger_tip.y" "")) 10.0) (* (`KismetStringLibrary.Conv_StringToDouble` (`EasyJsonObject.ReadString` _returnvalue "middle_finger_tip.z" "")) 10.0)) (struct) false false 0.0)
        (`KismetSystemLibrary.MoveComponentTo` (`self.ring_finger_mcp`) (`KismetMathLibrary.MakeVector` (* (`KismetStringLibrary.Conv_StringToDouble` (`EasyJsonObject.ReadString` _returnvalue "ring_finger_mcp.x" "")) 10.0) (* (`KismetStringLibrary.Conv_StringToDouble` (`EasyJsonObject.ReadString` _returnvalue "ring_finger_mcp.y" "")) 10.0) (* (`KismetStringLibrary.Conv_StringToDouble` (`EasyJsonObject.ReadString` _returnvalue "ring_finger_mcp.z" "")) 10.0)) (struct) false false 0.0)
        (`KismetSystemLibrary.MoveComponentTo` (`self.ring_finger_pip`) (`KismetMathLibrary.MakeVector` (* (`KismetStringLibrary.Conv_StringToDouble` (`EasyJsonObject.ReadString` _returnvalue "ring_finger_pip.x" "")) 10.0) (* (`KismetStringLibrary.Conv_StringToDouble` (`EasyJsonObject.ReadString` _returnvalue "ring_finger_pip.y" "")) 10.0) (* (`KismetStringLibrary.Conv_StringToDouble` (`EasyJsonObject.ReadString` _returnvalue "ring_finger_pip.z" "")) 10.0)) (struct) false false 0.0)
        (`KismetSystemLibrary.MoveComponentTo` (`self.ring_finger_dip`) (`KismetMathLibrary.MakeVector` (* (`KismetStringLibrary.Conv_StringToDouble` (`EasyJsonObject.ReadString` _returnvalue "ring_finger_dip.x" "")) 10.0) (* (`KismetStringLibrary.Conv_StringToDouble` (`EasyJsonObject.ReadString` _returnvalue "ring_finger_dip.y" "")) 10.0) (* (`KismetStringLibrary.Conv_StringToDouble` (`EasyJsonObject.ReadString` _returnvalue "ring_finger_dip.z" "")) 10.0)) (struct) false false 0.0)
        (`KismetSystemLibrary.MoveComponentTo` (`self.ring_finger_tip`) (`KismetMathLibrary.MakeVector` (* (`KismetStringLibrary.Conv_StringToDouble` (`EasyJsonObject.ReadString` _returnvalue "ring_finger_tip.x" "")) 10.0) (* (`KismetStringLibrary.Conv_StringToDouble` (`EasyJsonObject.ReadString` _returnvalue "ring_finger_tip.y" "")) 10.0) (* (`KismetStringLibrary.Conv_StringToDouble` (`EasyJsonObject.ReadString` _returnvalue "ring_finger_tip.z" "")) 10.0)) (struct) false false 0.0)
        (`KismetSystemLibrary.MoveComponentTo` (`self.pinky_mcp`) (`KismetMathLibrary.MakeVector` (* (`KismetStringLibrary.Conv_StringToDouble` (`EasyJsonObject.ReadString` _returnvalue "pinky_mcp.x" "")) 10.0) (* (`KismetStringLibrary.Conv_StringToDouble` (`EasyJsonObject.ReadString` _returnvalue "pinky_mcp.y" "")) 10.0) (* (`KismetStringLibrary.Conv_StringToDouble` (`EasyJsonObject.ReadString` _returnvalue "pinky_mcp.z" "")) 10.0)) (struct) false false 0.0)
        (`KismetSystemLibrary.MoveComponentTo` (`self.pinky_pip`) (`KismetMathLibrary.MakeVector` (* (`KismetStringLibrary.Conv_StringToDouble` (`EasyJsonObject.ReadString` _returnvalue "pinky_pip.x" "")) 10.0) (* (`KismetStringLibrary.Conv_StringToDouble` (`EasyJsonObject.ReadString` _returnvalue "pinky_pip.y" "")) 10.0) (* (`KismetStringLibrary.Conv_StringToDouble` (`EasyJsonObject.ReadString` _returnvalue "pinky_pip.z" "")) 10.0)) (struct) false false 0.0)
        (`KismetSystemLibrary.MoveComponentTo` (`self.pinky_dip`) (`KismetMathLibrary.MakeVector` (* (`KismetStringLibrary.Conv_StringToDouble` (`EasyJsonObject.ReadString` _returnvalue "pinky_dip.x" "")) 10.0) (* (`KismetStringLibrary.Conv_StringToDouble` (`EasyJsonObject.ReadString` _returnvalue "pinky_dip.y" "")) 10.0) (* (`KismetStringLibrary.Conv_StringToDouble` (`EasyJsonObject.ReadString` _returnvalue "pinky_dip.z" "")) 10.0)) (struct) false false 0.0)
        (`KismetSystemLibrary.MoveComponentTo` (`self.pinky_tip`) (`KismetMathLibrary.MakeVector` (* (`KismetStringLibrary.Conv_StringToDouble` (`EasyJsonObject.ReadString` _returnvalue "pinky_tip.x" "")) 10.0) (* (`KismetStringLibrary.Conv_StringToDouble` (`EasyJsonObject.ReadString` _returnvalue "pinky_tip.y" "")) 10.0) (* (`KismetStringLibrary.Conv_StringToDouble` (`EasyJsonObject.ReadString` _returnvalue "pinky_tip.z" "")) 10.0)) (struct) false false 0.0)
        (`KismetSystemLibrary.PrintString` (`KismetStringLibrary.BuildString_Int` "" "" (`SkinnedMeshComponent.GetNumBones` (`self.SkeletalMesh`))))))))

(fn `Init`
  (bind _skeletalmesh (`self.SkeletalMesh`))
  (bind _skeletalmesh_2 (`self.SkeletalMesh`))
  (bind _skeletalmesh_3 (`self.SkeletalMesh`))
  (bind _skeletalmesh_4 (`self.SkeletalMesh`))
  (bind _skeletalmesh_5 (`self.SkeletalMesh`))
  (bind _skeletalmesh_6 (`self.SkeletalMesh`))
  (bind _skeletalmesh_7 (`self.SkeletalMesh`))
  (bind _skeletalmesh_8 (`self.SkeletalMesh`))
  (bind _skeletalmesh_9 (`self.SkeletalMesh`))
  (bind _skeletalmesh_10 (`self.SkeletalMesh`))
  (bind _skeletalmesh_11 (`self.SkeletalMesh`))
  (bind _skeletalmesh_12 (`self.SkeletalMesh`))
  (bind _skeletalmesh_13 (`self.SkeletalMesh`))
  (bind _skeletalmesh_14 (`self.SkeletalMesh`))
  (bind _skeletalmesh_15 (`self.SkeletalMesh`))
  (bind _skeletalmesh_16 (`self.SkeletalMesh`))
  (bind _skeletalmesh_17 (`self.SkeletalMesh`))
  (bind _skeletalmesh_18 (`self.SkeletalMesh`))
  (bind _skeletalmesh_19 (`self.SkeletalMesh`))
  (bind _skeletalmesh_20 (`self.SkeletalMesh`))
  (bind _skeletalmesh_21 (`self.SkeletalMesh`))
  (`SkeletalMeshComponent.SetAllBodiesSimulatePhysics` _skeletalmesh_21 true)
  (for _array_element (`self.Mapping`)
    (`PrimitiveComponent.SetAngularDamping` _skeletalmesh_21 1000.0)
    (`PrimitiveComponent.SetLinearDamping` _skeletalmesh_21 1000.0)
    (bind _returnvalue (`|AddComponentByClass` "/Script/Engine.PhysicsHandleComponent"))
    (`|MultiGate` false
      (:`Out 1`
        (`PhysicsHandleComponent.GrabComponentAtLocation` _returnvalue _skeletalmesh "THUMB_CMC" (`SceneComponent.GetSocketLocation` _skeletalmesh "THUMB_CMC"))
        (`PhysicsHandleComponent.SetTargetLocation` _returnvalue (`SceneComponent.K2_GetComponentLocation` (`self.athumbcmc`)))
        (`PhysicsHandleComponent.SetTargetLocation` _returnvalue (`SceneComponent.K2_GetComponentLocation` (`self.athumbcmc`))))
      (:`Out 2`
        (`PhysicsHandleComponent.GrabComponentAtLocation` _returnvalue _skeletalmesh_4 "THUMB_MCP" (`SceneComponent.GetSocketLocation` _skeletalmesh_4 "THUMB_MCP"))
        (`PhysicsHandleComponent.SetTargetLocation` _returnvalue (`SceneComponent.K2_GetComponentLocation` (`self.athumbmcpm`))))
      (:`Out 3`
        (`PhysicsHandleComponent.GrabComponentAtLocation` _returnvalue _skeletalmesh_5 "THUMB_IP" (`SceneComponent.GetSocketLocation` _skeletalmesh_5 "THUMB_IP"))
        (`PhysicsHandleComponent.SetTargetLocation` _returnvalue (`SceneComponent.K2_GetComponentLocation` (`self.athumbip`))))
      (:`Out 4`
        (`PhysicsHandleComponent.GrabComponentAtLocation` _returnvalue _skeletalmesh_6 "THUMB_TIP" (`SceneComponent.GetSocketLocation` _skeletalmesh_6 "THUMB_TIP"))
        (`PhysicsHandleComponent.SetTargetLocation` _returnvalue (`SceneComponent.K2_GetComponentLocation` (`self.athumbtip`))))
      (:`Out 5`
        (`PhysicsHandleComponent.GrabComponentAtLocation` _returnvalue _skeletalmesh_7 "INDEX_FINGER_MCP" (`SceneComponent.GetSocketLocation` _skeletalmesh_7 "INDEX_FINGER_MCP"))
        (`PhysicsHandleComponent.SetTargetLocation` _returnvalue (`SceneComponent.K2_GetComponentLocation` (`self.aindexmcp1`))))
      (:`Out 6`
        (`PhysicsHandleComponent.GrabComponentAtLocation` _returnvalue _skeletalmesh_8 "INDEX_FINGER_PIP" (`SceneComponent.GetSocketLocation` _skeletalmesh_8 "INDEX_FINGER_PIP"))
        (`PhysicsHandleComponent.SetTargetLocation` _returnvalue (`SceneComponent.K2_GetComponentLocation` (`self.aindexpip`))))
      (:`Out 7`
        (`PhysicsHandleComponent.GrabComponentAtLocation` _returnvalue _skeletalmesh_9 "INDEX_FINGER_DIP" (`SceneComponent.GetSocketLocation` _skeletalmesh_9 "INDEX_FINGER_DIP"))
        (`PhysicsHandleComponent.SetTargetLocation` _returnvalue (`SceneComponent.K2_GetComponentLocation` (`self.aindexdip`))))
      (:`Out 8`
        (`PhysicsHandleComponent.GrabComponentAtLocation` _returnvalue _skeletalmesh_2 "INDEX_FINGER_TIP" (`SceneComponent.GetSocketLocation` _skeletalmesh_2 "INDEX_FINGER_TIP"))
        (`PhysicsHandleComponent.SetTargetLocation` _returnvalue (`SceneComponent.K2_GetComponentLocation` (`self.aindextip`))))
      (:`Out 9`
        (`PhysicsHandleComponent.GrabComponentAtLocation` _returnvalue _skeletalmesh_20 "MIDDLE_FINGER_MCP" (`SceneComponent.GetSocketLocation` _skeletalmesh_20 "MIDDLE_FINGER_MCP"))
        (`PhysicsHandleComponent.SetTargetLocation` _returnvalue (`SceneComponent.K2_GetComponentLocation` (`self.amiddlemcp`))))
      (:`Out 10`
        (`PhysicsHandleComponent.GrabComponentAtLocation` _returnvalue _skeletalmesh_10 "MIDDLE_FINGER_PIP" (`SceneComponent.GetSocketLocation` _skeletalmesh_10 "MIDDLE_FINGER_PIP"))
        (`PhysicsHandleComponent.SetTargetLocation` _returnvalue (`SceneComponent.K2_GetComponentLocation` (`self.amiddlepip`))))
      (:`Out 11`
        (`PhysicsHandleComponent.GrabComponentAtLocation` _returnvalue _skeletalmesh_11 "MIDDLE_FINGER_DIP" (`SceneComponent.GetSocketLocation` _skeletalmesh_11 "MIDDLE_FINGER_DIP"))
        (`PhysicsHandleComponent.SetTargetLocation` _returnvalue (`SceneComponent.K2_GetComponentLocation` (`self.amiddledip`))))
      (:`Out 12`
        (`PhysicsHandleComponent.GrabComponentAtLocation` _returnvalue _skeletalmesh_12 "MIDDLE_FINGER_TIP" (`SceneComponent.GetSocketLocation` _skeletalmesh_12 "MIDDLE_FINGER_TIP"))
        (`PhysicsHandleComponent.SetTargetLocation` _returnvalue (`SceneComponent.K2_GetComponentLocation` (`self.amiddletip`))))
      (:`Out 13`
        (`PhysicsHandleComponent.GrabComponentAtLocation` _returnvalue _skeletalmesh_13 "RING_FINGER_MCP" (`SceneComponent.GetSocketLocation` _skeletalmesh_13 "RING_FINGER_MCP"))
        (`PhysicsHandleComponent.SetTargetLocation` _returnvalue (`SceneComponent.K2_GetComponentLocation` (`self.aringmcp`))))
      (:`Out 14`
        (`PhysicsHandleComponent.GrabComponentAtLocation` _returnvalue _skeletalmesh_14 "RING_FINGER_PIP" (`SceneComponent.GetSocketLocation` _skeletalmesh_14 "RING_FINGER_PIP"))
        (`PhysicsHandleComponent.SetTargetLocation` _returnvalue (`SceneComponent.K2_GetComponentLocation` (`self.aringpip`))))
      (:`Out 15`
        (`PhysicsHandleComponent.GrabComponentAtLocation` _returnvalue _skeletalmesh_15 "RING_FINGER_DIP" (`SceneComponent.GetSocketLocation` _skeletalmesh_15 "RING_FINGER_DIP"))
        (`PhysicsHandleComponent.SetTargetLocation` _returnvalue (`SceneComponent.K2_GetComponentLocation` (`self.aringdip`))))
      (:`Out 16`
        (`PhysicsHandleComponent.GrabComponentAtLocation` _returnvalue _skeletalmesh_16 "RING_FINGER_TIP" (`SceneComponent.GetSocketLocation` _skeletalmesh_16 "RING_FINGER_TIP"))
        (`PhysicsHandleComponent.SetTargetLocation` _returnvalue (`SceneComponent.K2_GetComponentLocation` (`self.aringtip`))))
      (:`Out 17`
        (`PhysicsHandleComponent.GrabComponentAtLocation` _returnvalue _skeletalmesh_17 "PINKY_MCP" (`SceneComponent.GetSocketLocation` _skeletalmesh_17 "PINKY_MCP"))
        (`PhysicsHandleComponent.SetTargetLocation` _returnvalue (`SceneComponent.K2_GetComponentLocation` (`self.apinkymcp`))))
      (:`Out 18`
        (`PhysicsHandleComponent.GrabComponentAtLocation` _returnvalue _skeletalmesh_18 "PINKY_PIP" (`SceneComponent.GetSocketLocation` _skeletalmesh_18 "PINKY_PIP"))
        (`PhysicsHandleComponent.SetTargetLocation` _returnvalue (`SceneComponent.K2_GetComponentLocation` (`self.apinkypip`))))
      (:`Out 19`
        (`PhysicsHandleComponent.GrabComponentAtLocation` _returnvalue _skeletalmesh_19 "PINKY_DIP" (`SceneComponent.GetSocketLocation` _skeletalmesh_19 "PINKY_DIP"))
        (`PhysicsHandleComponent.SetTargetLocation` _returnvalue (`SceneComponent.K2_GetComponentLocation` (`self.apinkydip`))))
      (:`Out 20`
        (`PhysicsHandleComponent.GrabComponentAtLocation` _returnvalue _skeletalmesh_3 "PINKY_TIP" (`SceneComponent.GetSocketLocation` _skeletalmesh_3 "PINKY_TIP"))
        (`PhysicsHandleComponent.SetTargetLocation` _returnvalue (`SceneComponent.K2_GetComponentLocation` (`self.apinkytip`)))))))

(fn `UserConstructionScript`)