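; Actor wrapper around a MediaPipe pipeline that runs on a camera or file input and can display its video in the scene.
; StartPipe copies the input, capture, resolution, overlay and texture settings to the pipeline and starts it, only if EnableAutoStart is set; StopPipe stops it.
; When video texture is enabled, PipelineVideoTexture puts the new texture into a transient dynamic material on the Video component and makes it visible.
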(event `PipelineVideoTexture`
  (params (NewTexture :type "Texture2D Object Reference"))
  (bind _video (`self.Video`))
  (if (`self.EnableVideoTexture`)
    (bind _returnvalue (`KismetMaterialLibrary.CreateDynamicMaterialInstance` "/Game/Hand/Material__43.Material__43" "None" "Transient"))
    (`MaterialInstanceDynamic.SetTextureParameterValue` _returnvalue "Video" NewTexture)
    (`PrimitiveComponent.SetMaterial` _video 0 _returnvalue)
    (`SceneComponent.SetVisibility` _video true false)))

(fn `Start Pipe`
  (bind _mediapipepipeline (`self.MediaPipePipeline`))
  (if (`self.EnableAutoStart`)
    (set `MediaPipePipelineComponent.InputFile` (`self.InputFile`) _mediapipepipeline)
    (set `MediaPipePipelineComponent.CameraId` (`self.CamId`) _mediapipepipeline)
    (set `MediaPipePipelineComponent.CaptureApi` (`self.CaptureApi`) _mediapipepipeline)
    (set `MediaPipePipelineComponent.ResX` (`self.ResX`) _mediapipepipeline)
    (set `MediaPipePipelineComponent.ResY` (`self.ResY`) _mediapipepipeline)
    (set `MediaPipePipelineComponent.bEnableOverlay` (`self.EnableOverlay`) _mediapipepipeline)
    (set `MediaPipePipelineComponent.bEnableVideoTexture` (`self.EnableVideoTexture`) _mediapipepipeline)
    (`MediaPipePipelineComponent.Start` _mediapipepipeline)))

(fn `StopPipe`
  (`MediaPipePipelineComponent.Stop` (`self.MediaPipePipeline`)))

(fn `UserConstructionScript`)