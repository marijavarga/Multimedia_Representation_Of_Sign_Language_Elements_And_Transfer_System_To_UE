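; Socket actor that drives a physics-simulated skeletal hand from landmark data received over SocketIO.
; Each "new wind" JSON message is parsed and moves per-joint components to scaled positions, with X and Y swapped for index and middle fingers.
; Init runs every Tick, enabling physics and adding a PhysicsHandle per Mapping entry that grabs the wrist, then index tip bone, targeting those components.
; Other physics and offset snippets are unconnected.
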(event `self.ReceiveBeginPlay`
  (`SocketIOClientComponent.BindEventToGenericEvent` (`self.SocketIOClient`) "new wind" "/"))

(event `self.ReceiveTick`
  (params (DeltaSeconds :type "Float (single-precision)"))
  (`self.Init`))

(event `self.SocketIOClient.OnConnected`
  (params (SessionId :type String) (bIsReconnection :type Boolean))
  (`KismetSystemLibrary.PrintString` "Connected"))

(event `self.SocketIOClient.OnDisconnected`
  (params (Reason :type "ESIOConnectionCloseReason Enum" :default "CLOSE_REASON_NORMAL"))
  (`KismetSystemLibrary.PrintString` (`KismetStringLibrary.Concat_StrStr` "Disconnected" (`|GetEnumeratorNameAsString` Reason))))

(event `self.SocketIOClient.OnGenericEvent`
  (params (EventName :type String) (MessageJson :type "SIOJsonValue Object Reference"))
  ;[1 1 1] SocketIO i EasyJsonParser plaginovi
  (if (`KismetStringLibrary.EqualEqual_StrStr` EventName "new wind")
    (bind _returnvalue (`EasyJsonParseManager.LoadFromString` (`SIOJsonValue.AsString` MessageJson))
      (:`Successed`
        (`KismetSystemLibrary.PrintString` "Hello")
        (bind _returnvalue_2 (`KismetMathLibrary.MakeVector` (* (`KismetStringLibrary.Conv_StringToDouble` (`EasyJsonObject.ReadString` _returnvalue "wrist.x" "")) 2.0) (* (`KismetStringLibrary.Conv_StringToDouble` (`EasyJsonObject.ReadString` _returnvalue "wrist.y" "")) 2.0) (* (`KismetStringLibrary.Conv_StringToDouble` (`EasyJsonObject.ReadString` _returnvalue "wrist.z" "")) 2.0)))
        (bind _returnvalue_3 (* (`KismetStringLibrary.Conv_StringToDouble` (`EasyJsonObject.ReadString` _returnvalue "index_finger_tip.x" "")) 2.0))
        (`KismetSystemLibrary.MoveComponentTo` (`self.wrist`) _returnvalue_2 (* (`KismetMathLibrary.MakeRotationFromAxes` _returnvalue_2 (`KismetMathLibrary.Conv_DoubleToVector` _returnvalue_3)) 1) false false 0.0)
        (`KismetSystemLibrary.MoveComponentTo` (`self.thumb_cmc`) (`KismetMathLibrary.MakeVector` (* (`KismetStringLibrary.Conv_StringToDouble` (`EasyJsonObject.ReadString` _returnvalue "thumb_cmc.x" "")) 2.0) (* (`KismetStringLibrary.Conv_StringToDouble` (`EasyJsonObject.ReadString` _returnvalue "thumb_cmc.y" "")) 2.0) (* (`KismetStringLibrary.Conv_StringToDouble` (`EasyJsonObject.ReadString` _returnvalue "thumb_cmc.z" "")) 2.0)) (struct) false false 0.0)
        (`KismetSystemLibrary.MoveComponentTo` (`self.thumb_mcp`) (`KismetMathLibrary.MakeVector` (* (`KismetStringLibrary.Conv_StringToDouble` (`EasyJsonObject.ReadString` _returnvalue "thumb_mcp.x" "")) 2.0) (* (`KismetStringLibrary.Conv_StringToDouble` (`EasyJsonObject.ReadString` _returnvalue "thumb_mcp.y" "")) 2.0) (* (`KismetStringLibrary.Conv_StringToDouble` (`EasyJsonObject.ReadString` _returnvalue "thumb_mcp.z" "")) 2.0)) (struct) false false 0.0)
        (`KismetSystemLibrary.MoveComponentTo` (`self.thumb_ip`) (`KismetMathLibrary.MakeVector` (* (`KismetStringLibrary.Conv_StringToDouble` (`EasyJsonObject.ReadString` _returnvalue "thumb_ip.x" "")) 2.0) (* (`KismetStringLibrary.Conv_StringToDouble` (`EasyJsonObject.ReadString` _returnvalue "thumb_ip.y" "")) 2.0) (* (`KismetStringLibrary.Conv_StringToDouble` (`EasyJsonObject.ReadString` _returnvalue "thumb_ip.z" "")) 2.0)) (struct) false false 0.0)
        (`KismetSystemLibrary.MoveComponentTo` (`self.thumb_tip`) (`KismetMathLibrary.MakeVector` (* (`KismetStringLibrary.Conv_StringToDouble` (`EasyJsonObject.ReadString` _returnvalue "thumb_tip.x" "")) 2.0) (* (`KismetStringLibrary.Conv_StringToDouble` (`EasyJsonObject.ReadString` _returnvalue "thumb_tip.y" "")) 2.0) (* (`KismetStringLibrary.Conv_StringToDouble` (`EasyJsonObject.ReadString` _returnvalue "thumb_tip.z" "")) 2.0)) (struct) false false 0.0)
        (`KismetSystemLibrary.MoveComponentTo` (`self.index_finger_mcp`) (`KismetMathLibrary.MakeVector` (* (`KismetStringLibrary.Conv_StringToDouble` (`EasyJsonObject.ReadString` _returnvalue "index_finger_mcp.y" "")) 2.0) (* (`KismetStringLibrary.Conv_StringToDouble` (`EasyJsonObject.ReadString` _returnvalue "index_finger_mcp.x" "")) 2.0) (* (`KismetStringLibrary.Conv_StringToDouble` (`EasyJsonObject.ReadString` _returnvalue "index_finger_mcp.z" "")) 2.0)) (struct) false false 0.0)
        (`KismetSystemLibrary.MoveComponentTo` (`self.index_finger_pip`) (`KismetMathLibrary.MakeVector` (* (`KismetStringLibrary.Conv_StringToDouble` (`EasyJsonObject.ReadString` _returnvalue "index_finger_pip.y" "")) 2.0) (* (`KismetStringLibrary.Conv_StringToDouble` (`EasyJsonObject.ReadString` _returnvalue "index_finger_pip.x" "")) 2.0) (* (`KismetStringLibrary.Conv_StringToDouble` (`EasyJsonObject.ReadString` _returnvalue "index_finger_pip.z" "")) 2.0)) (struct) false false 0.0)
        (`KismetSystemLibrary.MoveComponentTo` (`self.index_finger_dip`) (`KismetMathLibrary.MakeVector` (* (`KismetStringLibrary.Conv_StringToDouble` (`EasyJsonObject.ReadString` _returnvalue "index_finger_dip.y" "")) 2.0) (* (`KismetStringLibrary.Conv_StringToDouble` (`EasyJsonObject.ReadString` _returnvalue "index_finger_dip.x" "")) 2.0) (* (`KismetStringLibrary.Conv_StringToDouble` (`EasyJsonObject.ReadString` _returnvalue "index_finger_dip.z" "")) 2.0)) (struct) false false 0.0)
        (`KismetSystemLibrary.MoveComponentTo` (`self.index_finger_tip`) (`KismetMathLibrary.MakeVector` (* (`KismetStringLibrary.Conv_StringToDouble` (`EasyJsonObject.ReadString` _returnvalue "index_finger_tip.y" "")) 2.0) _returnvalue_3 (* (`KismetStringLibrary.Conv_StringToDouble` (`EasyJsonObject.ReadString` _returnvalue "index_finger_tip.z" "")) 2.0)) (struct) false false 0.0)
        (`KismetSystemLibrary.MoveComponentTo` (`self.middle_finger_mcp`) (`KismetMathLibrary.MakeVector` (* (`KismetStringLibrary.Conv_StringToDouble` (`EasyJsonObject.ReadString` _returnvalue "middle_finger_mcp.y" "")) 2.0) (* (`KismetStringLibrary.Conv_StringToDouble` (`EasyJsonObject.ReadString` _returnvalue "middle_finger_mcp.x" "")) 2.0) (* (`KismetStringLibrary.Conv_StringToDouble` (`EasyJsonObject.ReadString` _returnvalue "middle_finger_mcp.z" "")) 2.0)) (struct) false false 0.0)
        (`KismetSystemLibrary.MoveComponentTo` (`self.middle_finger_pip`) (`KismetMathLibrary.MakeVector` (* (`KismetStringLibrary.Conv_StringToDouble` (`EasyJsonObject.ReadString` _returnvalue "middle_finger_pip.y" "")) 2.0) (* (`KismetStringLibrary.Conv_StringToDouble` (`EasyJsonObject.ReadString` _returnvalue "middle_finger_pip.x" "")) 2.0) (* (`KismetStringLibrary.Conv_StringToDouble` (`EasyJsonObject.ReadString` _returnvalue "middle_finger_pip.z" "")) 2.0)) (struct) false false 0.0)
        (`KismetSystemLibrary.MoveComponentTo` (`self.middle_finger_dip`) (`KismetMathLibrary.MakeVector` (* (`KismetStringLibrary.Conv_StringToDouble` (`EasyJsonObject.ReadString` _returnvalue "middle_finger_dip.y" "")) 2.0) (* (`KismetStringLibrary.Conv_StringToDouble` (`EasyJsonObject.ReadString` _returnvalue "middle_finger_dip.x" "")) 2.0) (* (`KismetStringLibrary.Conv_StringToDouble` (`EasyJsonObject.ReadString` _returnvalue "middle_finger_dip.z" "")) 2.0)) (struct) false false 0.0)
        (`KismetSystemLibrary.MoveComponentTo` (`self.middle_finger_tip`) (`KismetMathLibrary.MakeVector` (* (`KismetStringLibrary.Conv_StringToDouble` (`EasyJsonObject.ReadString` _returnvalue "middle_finger_tip.y" "")) 2.0) (* (`KismetStringLibrary.Conv_StringToDouble` (`EasyJsonObject.ReadString` _returnvalue "middle_finger_tip.x" "")) 2.0) (* (`KismetStringLibrary.Conv_StringToDouble` (`EasyJsonObject.ReadString` _returnvalue "middle_finger_tip.z" "")) 2.0)) (struct) false false 0.0)
        (`KismetSystemLibrary.MoveComponentTo` (`self.ring_finger_mcp`) (`KismetMathLibrary.MakeVector` (* (`KismetStringLibrary.Conv_StringToDouble` (`EasyJsonObject.ReadString` _returnvalue "ring_finger_mcp.x" "")) 2.0) (* (`KismetStringLibrary.Conv_StringToDouble` (`EasyJsonObject.ReadString` _returnvalue "ring_finger_mcp.y" "")) 2.0) (* (`KismetStringLibrary.Conv_StringToDouble` (`EasyJsonObject.ReadString` _returnvalue "ring_finger_mcp.z" "")) 2.0)) (struct) false false 0.0)
        (`KismetSystemLibrary.MoveComponentTo` (`self.ring_finger_pip`) (`KismetMathLibrary.MakeVector` (* (`KismetStringLibrary.Conv_StringToDouble` (`EasyJsonObject.ReadString` _returnvalue "ring_finger_pip.x" "")) 2.0) (* (`KismetStringLibrary.Conv_StringToDouble` (`EasyJsonObject.ReadString` _returnvalue "ring_finger_pip.y" "")) 2.0) (* (`KismetStringLibrary.Conv_StringToDouble` (`EasyJsonObject.ReadString` _returnvalue "ring_finger_pip.z" "")) 2.0)) (struct) false false 0.0)
        (`KismetSystemLibrary.MoveComponentTo` (`self.ring_finger_dip`) (`KismetMathLibrary.MakeVector` (* (`KismetStringLibrary.Conv_StringToDouble` (`EasyJsonObject.ReadString` _returnvalue "ring_finger_dip.x" "")) 5.0) (* (`KismetStringLibrary.Conv_StringToDouble` (`EasyJsonObject.ReadString` _returnvalue "ring_finger_dip.y" "")) 5.0) (* (`KismetStringLibrary.Conv_StringToDouble` (`EasyJsonObject.ReadString` _returnvalue "ring_finger_dip.z" "")) 5.0)) (struct) false false 0.0)
        (`KismetSystemLibrary.MoveComponentTo` (`self.ring_finger_tip`) (`KismetMathLibrary.MakeVector` (* (`KismetStringLibrary.Conv_StringToDouble` (`EasyJsonObject.ReadString` _returnvalue "ring_finger_tip.x" "")) 2.0) (* (`KismetStringLibrary.Conv_StringToDouble` (`EasyJsonObject.ReadString` _returnvalue "ring_finger_tip.y" "")) 2.0) (* (`KismetStringLibrary.Conv_StringToDouble` (`EasyJsonObject.ReadString` _returnvalue "ring_finger_tip.z" "")) 2.0)) (struct) false false 0.0)
        (`KismetSystemLibrary.MoveComponentTo` (`self.pinky_mcp`) (`KismetMathLibrary.MakeVector` (* (`KismetStringLibrary.Conv_StringToDouble` (`EasyJsonObject.ReadString` _returnvalue "pinky_mcp.x" "")) 2.0) (* (`KismetStringLibrary.Conv_StringToDouble` (`EasyJsonObject.ReadString` _returnvalue "pinky_mcp.y" "")) 2.0) (* (`KismetStringLibrary.Conv_StringToDouble` (`EasyJsonObject.ReadString` _returnvalue "pinky_mcp.z" "")) 2.0)) (struct) false false 0.0)
        (`KismetSystemLibrary.MoveComponentTo` (`self.pinky_pip`) (`KismetMathLibrary.MakeVector` (* (`KismetStringLibrary.Conv_StringToDouble` (`EasyJsonObject.ReadString` _returnvalue "pinky_pip.x" "")) 2.0) (* (`KismetStringLibrary.Conv_StringToDouble` (`EasyJsonObject.ReadString` _returnvalue "pinky_pip.y" "")) 2.0) (* (`KismetStringLibrary.Conv_StringToDouble` (`EasyJsonObject.ReadString` _returnvalue "pinky_pip.z" "")) 2.0)) (struct) false false 0.0)
        (`KismetSystemLibrary.MoveComponentTo` (`self.pinky_dip`) (`KismetMathLibrary.MakeVector` (* (`KismetStringLibrary.Conv_StringToDouble` (`EasyJsonObject.ReadString` _returnvalue "pinky_dip.x" "")) 2.0) (* (`KismetStringLibrary.Conv_StringToDouble` (`EasyJsonObject.ReadString` _returnvalue "pinky_dip.y" "")) 2.0) (* (`KismetStringLibrary.Conv_StringToDouble` (`EasyJsonObject.ReadString` _returnvalue "pinky_dip.z" "")) 2.0)) (struct) false false 0.0)
        (`KismetSystemLibrary.MoveComponentTo` (`self.pinky_tip`) (`KismetMathLibrary.MakeVector` (* (`KismetStringLibrary.Conv_StringToDouble` (`EasyJsonObject.ReadString` _returnvalue "pinky_tip.x" "")) 2.0) (* (`KismetStringLibrary.Conv_StringToDouble` (`EasyJsonObject.ReadString` _returnvalue "pinky_tip.y" "")) 2.0) (* (`KismetStringLibrary.Conv_StringToDouble` (`EasyJsonObject.ReadString` _returnvalue "pinky_tip.z" "")) 2.0)) (struct) false false 0.0)
        (`KismetSystemLibrary.PrintString` (`KismetStringLibrary.BuildString_Int` "" "" (`SkinnedMeshComponent.GetNumBones` (`self.SkeletalMesh`))))))))

(fn `Init`
  (bind _skeletalmesh (`self.SkeletalMesh`))
  (bind _skeletalmesh_2 (`self.SkeletalMesh`))
  (`SkeletalMeshComponent.SetAllBodiesSimulatePhysics` (`self.SkeletalMesh`) true)
  (for _array_element (`self.Mapping`)
    (bind _returnvalue (`|AddComponentByClass` "/Script/Engine.PhysicsHandleComponent"))
    (`BlueprintMapLibrary.Map_Add` (`self.grabbers`) (`.StringName_22_5AB1459947AAB7B7650CF1A74C37588F` (break `/Game/Blueprint/BoneMap` _array_element)) _returnvalue)
    (`PhysicsHandleComponent.GrabComponentAtLocation` _returnvalue _skeletalmesh "WRIST" (`SceneComponent.GetSocketLocation` _skeletalmesh "WRIST"))
    (`PhysicsHandleComponent.SetTargetLocation` _returnvalue (`SceneComponent.K2_GetComponentLocation` (`self.wrist`)))
    (`PhysicsHandleComponent.GrabComponentAtLocation` _returnvalue _skeletalmesh_2 "INDEX_FINGER_TIP" (`SceneComponent.GetSocketLocation` _skeletalmesh_2 "INDEX_FINGER_TIP"))
    (`PhysicsHandleComponent.SetTargetLocation` _returnvalue (`SceneComponent.K2_GetComponentLocation` (`self.index_finger_tip`)))))

(fn `UserConstructionScript`)